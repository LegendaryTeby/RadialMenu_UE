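; Player character Blueprint that drives radial menu widgets from gamepad or mouse input.
; BeginPlay creates BP_RadialWidget_2, which holds center and corner radials; creation of the single BP_RadialWidget is never called.
; Tick feeds both radials either stored stick axes or raw cursor position, depending on IsGamepad.
; The SelectRadial input action confirms selection on both, while the single-widget update and select paths remain wired behind validity checks.
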(event Input|EnhancedActionEvents|EnhancedInputActionGamepadRadial_X
  (params (ActionValue :type Float%20%28double-precision%29) (ElapsedSeconds :type Float%20%28double-precision%29) (TriggeredSeconds :type Float%20%28double-precision%29) (InputAction :type Input%20Action%20Object%20Reference :default "/Game/Inputs/GamepadRadial_X.GamepadRadial_X"))
  ;[1 1 1] Gamepad Y Axis Value
  (:Triggered
    (Variables|Values|SetX ActionValue)))

(event Input|EnhancedActionEvents|EnhancedInputActionGamepadRadial_Y
  (params (ActionValue :type Float%20%28double-precision%29) (ElapsedSeconds :type Float%20%28double-precision%29) (TriggeredSeconds :type Float%20%28double-precision%29) (InputAction :type Input%20Action%20Object%20Reference :default "/Game/Inputs/GamepadRadial_Y.GamepadRadial_Y"))
  ;[1 1 1] Gamepad X Axis Value
  (:Triggered
    (Variables|Values|SetY ActionValue)))

(event Input|EnhancedActionEvents|EnhancedInputActionSelectRadial
  (params (ActionValue :type Boolean) (ElapsedSeconds :type Float%20%28double-precision%29) (TriggeredSeconds :type Float%20%28double-precision%29) (InputAction :type Input%20Action%20Object%20Reference :default "/Game/Inputs/SelectRadial.SelectRadial"))
  (:Triggered
    (CallFunction|SelectRadialWidget)
    (CallFunction|SelectRadialWidget2)))

(event EventBeginPlay
  (CallFunction|CreateRadialWidget2))

(event EventTick
  (params (DeltaSeconds :type Float%20%28single-precision%29))
  (CallFunction|UpdateRadialWidget)
  (CallFunction|UpdateRadialWidget2))

(fn ConstructionScript)

(fn CreateRadialWidget
  (bind _returnvalue (UserInterface|CreateWidget "/Game/Blueprint/HUD/BP_RadialWidget.BP_RadialWidget_C"))
  (bind _output_get (Variables|Widget|SetRadial%20Widget _returnvalue))
  (UserInterface|Viewport|AddtoViewport _output_get 0))

(fn CreateRadialWidget2
  (bind _returnvalue (UserInterface|CreateWidget "/Game/Blueprint/HUD/BP_RadialWidget_2.BP_RadialWidget_2_C"))
  (bind _output_get (Variables|Widget|SetRadial%20Widget_2 _returnvalue))
  (UserInterface|Viewport|AddtoViewport _output_get 0))

(fn UpdateRadialWidget
  (bind _returnvalue (Game|GetPlayerController 0))
  (bind (_locationx _locationy) (Game|Player|GetMousePosition _returnvalue))
  (Utilities|IsValid (Variables|Widget|GetRadial%20Widget)
    (:Is%20Valid
      (if (Variables|Values|GetIs%20Gamepad)
        ;[1 1 1] Controller
        (Class|RadialWidget|UpdateRadialWidget (Variables|Widget|GetRadial%20Widget) (Variables|Values|GetX) (Variables|Values|GetY))
        (else
          ;[1 1 1] Mouse Cursor
          (Class|RadialWidget|UpdateRadialWidgetRaw (Variables|Widget|GetRadial%20Widget) _locationx _locationy))))))

(fn UpdateRadialWidget2
  (bind _returnvalue (Game|GetPlayerController 0))
  (bind _x (Variables|Values|GetX))
  (bind _y (Variables|Values|GetY))
  (bind _radial_widget_2 (Variables|Widget|GetRadial%20Widget_2))
  (bind (_locationx _locationy) (Game|Player|GetMousePosition _returnvalue))
  (Utilities|IsValid (Variables|Widget|GetRadial%20Widget_2)
    (:Is%20Valid
      (LocalVariables|SetRadial%20Widget%20Center (Variables|/Game/Blueprint/HUD/BP_RadialWidget_2.BP_RadialWidget_2_C|GetRadialWidgetCenter _radial_widget_2))
      (LocalVariables|SetRadial%20Widget%20Corner (Variables|/Game/Blueprint/HUD/BP_RadialWidget_2.BP_RadialWidget_2_C|GetRadialWidgetCorner _radial_widget_2))
      (if (and (Utilities|IsValid (LocalVariables|GetRadial%20Widget%20Center)) (Utilities|IsValid (LocalVariables|GetRadial%20Widget%20Center)))
        (if (Variables|Values|GetIs%20Gamepad)
          ;[1 1 1] Controller
          (Class|RadialWidget|UpdateRadialWidget (LocalVariables|GetRadial%20Widget%20Center) _x _y)
          (Class|RadialWidget|UpdateRadialWidget (LocalVariables|GetRadial%20Widget%20Corner) _x _y)
          (else
            (Class|RadialWidget|UpdateRadialWidgetRaw (LocalVariables|GetRadial%20Widget%20Center) _locationx _locationy)
            (Class|RadialWidget|UpdateRadialWidgetRaw (LocalVariables|GetRadial%20Widget%20Corner) _locationx _locationy)))))))

(fn SelectRadialWidget
  (bind _radial_widget (Variables|Widget|GetRadial%20Widget))
  (Utilities|IsValid _radial_widget
    (:Is%20Valid
      (Class|RadialWidget|SelectRadial _radial_widget))))

(fn SelectRadialWidget2
  (bind _radial_widget_2 (Variables|Widget|GetRadial%20Widget_2))
  (Utilities|IsValid (Variables|Widget|GetRadial%20Widget_2)
    (:Is%20Valid
      (LocalVariables|SetRadial%20Widget%20Center (Variables|/Game/Blueprint/HUD/BP_RadialWidget_2.BP_RadialWidget_2_C|GetRadialWidgetCenter _radial_widget_2))
      (LocalVariables|SetRadial%20Widget%20Corner (Variables|/Game/Blueprint/HUD/BP_RadialWidget_2.BP_RadialWidget_2_C|GetRadialWidgetCorner _radial_widget_2))
      (if (and (Utilities|IsValid (LocalVariables|GetRadial%20Widget%20Center)) (Utilities|IsValid (LocalVariables|GetRadial%20Widget%20Center)))
        (Class|RadialWidget|SelectRadial (LocalVariables|GetRadial%20Widget%20Corner))
        (Class|RadialWidget|SelectRadial (LocalVariables|GetRadial%20Widget%20Center))))))